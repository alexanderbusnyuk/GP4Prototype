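; AC_Mover is a reusable component that slides an assigned scene component between two relative locations at a given rate.
; Initialize sets the component to move, and StartMoving stores the endpoints and speed, resets progress and enables Tick, ignoring calls made mid-move.
; Tick advances a linear lerp without sweep, snaps to the target on completion, disables itself and flags AtTargetPosition.
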(event `self.ReceiveTick`
  (params (DeltaSeconds :type "Float (single-precision)"))
  (`SceneComponent.K2_SetRelativeLocation` (`self.Component`) (`KismetMathLibrary.VLerp` (`self.Starting Location`) (`self.Target Location`) (`self.LerpProgress`)) false false)
  (bind _output_get (set `self.LerpProgress` (+ (`self.LerpProgress`) (* (`self.LerpSpeed`) DeltaSeconds))))
  (if (>= _output_get 1.0)
    (if (not (== (`SceneComponent.RelativeLocation` (`self.Component`)) (`self.Target Location`)))
      (`SceneComponent.K2_SetRelativeLocation` (`self.Component`) (`self.Target Location`) false false))
    (`self.SetComponentTickEnabled` false)
    (set `self.Moving` false)
    (set `self.AtTargetPosition` true)))

(fn `Initialize`
  (params (`Target Component` :type "SceneComponent Object Reference"))
  (set `self.Component` `Target Component`))

(fn `StartMoving`
  (params (Speed :type "Float (double-precision)") (StartingPosition :type "Vector Structure") (TargetPosition :type "Vector Structure"))
  (locals (IntermediateTarget :type "Vector Structure"))
  (if (not (`self.Moving`))
    (`self.SetVariables` Speed StartingPosition TargetPosition)
    (`self.SetComponentTickEnabled` true)
    (set `self.Moving` true)
    (set `self.AtTargetPosition` false)))