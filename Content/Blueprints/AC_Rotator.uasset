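; Actor component that rotates a scene component from a start to a target relative rotation over time.
; Initialize assigns the component, and StartRotating stores speed and rotations, snaps to the start, then enables tick, ignoring calls while already moving.
; Tick lerps the rotation by accumulated progress, then snaps to the target, disables its own tick and flags arrival.
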(event `self.ReceiveTick`
  (params (DeltaSeconds :type "Float (single-precision)"))
  (`SceneComponent.K2_SetRelativeRotation` (`self.Component`) (`KismetMathLibrary.RLerp` (`self.StartingRotation`) (`self.TargetRotation`) (`self.LerpProgress`)) false false)
  (bind _output_get (set `self.LerpProgress` (+ (`self.LerpProgress`) (* (`self.LerpSpeed`) DeltaSeconds))))
  (if (> _output_get 1.0)
    (if (not (== (`SceneComponent.RelativeRotation` (`self.Component`)) (`self.TargetRotation`)))
      (`SceneComponent.K2_SetRelativeRotation` (`self.Component`) (`self.TargetRotation`) false false))
    (`self.SetComponentTickEnabled` false)
    (set `self.Moving` false)
    (set `self.AtTargetPosition` true)))

(fn `Initialize`
  (params (TargetComponent :type "SceneComponent Object Reference"))
  (set `self.Component` TargetComponent))

(fn `StartRotating`
  (params (Speed :type "Float (double-precision)") (StartingRotation :type "Rotator Structure") (TargetRotation :type "Rotator Structure"))
  (locals (IntermediateTarget :type "Vector Structure"))
  (if (not (`self.Moving`))
    (`self.SetVariables` Speed StartingRotation TargetRotation)
    (`SceneComponent.K2_SetRelativeRotation` (`self.Component`) (`self.StartingRotation`) false false)
    (`self.SetComponentTickEnabled` true)
    (set `self.Moving` true)
    (set `self.AtTargetPosition` false)))