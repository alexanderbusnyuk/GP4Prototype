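; Parent Blueprint for interactable objects that can distract, electrocute or be boobytrapped, with hover prompts for each action.
; Interact from anything but BP_ThirdPersonCharacter sends DistractMessage to actors found by a sphere trace; from that character, it triggers Overload if boobytrapped.
; Overload spends GameMode energy and, on success, ragdolls actors within the electrocution radius and clears any trap.
; Boobytrap toggles the trap, registering or removing it with the GameMode.
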(event `/Game/Blueprints/BI_Interactable.InteractStart`
  (params (TriggeringActor :type "Actor Object Reference") (TypeOfInteraction :type "/Game/Blueprints/Enum_InteractionType Enum" :default "NewEnumerator0"))
  (bind _returnvalue (`self.K2_GetActorLocation`))
  (bind _gamemode (`self.GameMode`))
  (set `self.CharacterInteracting` (== (`GameplayStatics.GetObjectClass` TriggeringActor) "/Game/Blueprints/Characters/BP_ThirdPersonCharacter.BP_ThirdPersonCharacter_C"))
  (set `self.TypeOfInteraction` TypeOfInteraction)
  (switch `/Game/Blueprints/Enum_InteractionType` (`self.TypeOfInteraction`)
    (:`NewEnumerator0`
      (if (`self.Boobytrapped`)
        (if (`self.CharacterInteracting`)
          (`self.InteractStart` null "NewEnumerator1")
          (else
            (set `self.Overload` false :!label _label)
            (set `self.SphereRadius` (`self.DistractionRadius`))
            (bind _outhits (`KismetSystemLibrary.SphereTraceMulti` :`Start` _returnvalue :`End` _returnvalue :`Radius` (`self.SphereRadius`) :`TraceChannel` "TraceTypeQuery4" :`DrawDebugType` "Persistent" :!label _label_2))
            (for _array_element _outhits
              (switch `/Game/Blueprints/Enum_InteractionType` (`self.TypeOfInteraction`)
                (:`NewEnumerator0`
                  (bind (_bblockinghit _binitialoverlap _time _distance _location _impactpoint _normal _impactnormal _physmat _hitactor) (`GameplayStatics.BreakHitResult` _array_element))
                  (message `/Game/Blueprints/BI_Character.Distract` _hitactor true (`self.K2_GetActorLocation`)))
                (:`NewEnumerator1`
                  (if (`self.OverloadSuccess`)
                    (message `/Game/Blueprints/BI_Ragdoll.EnableRagdoll` _hitactor (0.0 0.0 0.0))
                    (if (`self.Boobytrapped`)
                      (`/Game/ThirdPerson/Blueprints/BP_ThirdPersonGameMode.RemoveBoobytrapSource` (`self.GameMode`))
                      (set `self.Boobytrapped` false))))))))
        (elif (not (`self.CharacterInteracting`))
          (goto _label))))
    (:`NewEnumerator1`
      (set `self.Overload` true)
      (set `self.SphereRadius` (`self.ElectrocutionRadius`))
      (bind _success (`/Game/ThirdPerson/Blueprints/BP_ThirdPersonGameMode.TryUseEnergy` (`self.GameMode`) (`self.OverloadCost`)))
      (set `self.OverloadSuccess` _success)
      (goto _label_2))
    (:`NewEnumerator2`
      (if (`self.Boobytrapped`)
        (`/Game/ThirdPerson/Blueprints/BP_ThirdPersonGameMode.RemoveBoobytrapSource` _gamemode)
        (set `self.Boobytrapped` false)
        (else
          (`/Game/ThirdPerson/Blueprints/BP_ThirdPersonGameMode.AddBoobytrapSource` _gamemode)
          (set `self.Boobytrapped` true))))))

(fn `GetHoverText`
  (returns (InteractText :type String) (OverloadText :type String) (BoobytrapText :type String))
  (return "Press [E] to distract" "Press [E] to electrocute" "Press [E] to boobytrap"))

(fn `Initialize`
  (params (DistractionRadius :type "Float (double-precision)") (Sound :type "SoundBase Object Reference"))
  (set `self.DistractionRadius` DistractionRadius)
  (set `self.Sound` Sound)
  (bind _asbp_third_person_game_mode (cast `/Game/ThirdPerson/Blueprints/BP_ThirdPersonGameMode` (`GameplayStatics.GetGameMode`)))
  (set `self.GameMode` _asbp_third_person_game_mode))

(fn `IsInteractableThroughWalls`
  (returns (InteractableThroughWalls :type Boolean))
  (return false))

(fn `UserConstructionScript`)