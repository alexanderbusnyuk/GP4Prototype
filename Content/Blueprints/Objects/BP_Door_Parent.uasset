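; Parent door actor that the player's camera or characters can swing open or closed, with characters limited to opening.
; TriggerOpen drives a rotator component to swing away from the triggering actor's nearer side, and Tick updates the open state on arrival.
; Overload spends game-mode energy for a faster swing that ragdolls characters it hits.
; Player use briefly blocks character interaction; boobytrap logic is disconnected, though its hover text remains.
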(event `self.ReceiveBeginPlay`
  (`/Game/Blueprints/AC_Rotator.Initialize` (`self.AC_Rotator`) (`self.SM_Bld_Door_01`))
  (bind _asbp_third_person_game_mode (cast `/Game/ThirdPerson/Blueprints/BP_ThirdPersonGameMode` (`GameplayStatics.GetGameMode`)))
  (set `self.GameMode` _asbp_third_person_game_mode))

(event `self.ReceiveTick`
  (params (DeltaSeconds :type "Float (single-precision)"))
  (bind (_relativerotation_roll _relativerotation_pitch _relativerotation_yaw) (`KismetMathLibrary.BreakRotator` (`SceneComponent.RelativeRotation` (`self.SM_Bld_Door_01`))))
  (if (`self.DoorStatusUpdated`)
    _
    (elif (== _relativerotation_yaw (`self.TargetRotation`))
      (if (== (`KismetMathLibrary.Abs` _relativerotation_yaw) (`self.MaxRotation`))
        (set `self.DoorOpen` true)
        (else
          (set `self.DoorOpen` false)))
      (set `self.DoorStatusUpdated` true))))

(event `self.Left.OnComponentHit`
  (params (HitComponent :type "PrimitiveComponent Object Reference") (OtherActor :type "Actor Object Reference") (OtherComp :type "PrimitiveComponent Object Reference") (NormalImpulse :type "Vector Structure") (Hit :type "HitResult Structure (by ref)"))
  (if (and (`self.Overloaaded`) (`/Game/Blueprints/AC_Rotator.Moving` (`self.AC_Rotator`)) (== (`GameplayStatics.GetObjectClass` OtherActor) "/Game/Blueprints/Characters/BP_ThirdPersonCharacter.BP_ThirdPersonCharacter_C"))
    (message `/Game/Blueprints/BI_Ragdoll.EnableRagdoll` OtherActor (`SceneComponent.GetForwardVector` (`self.SM_Bld_Door_01`)))))

(event `self.Right.OnComponentHit`
  (params (HitComponent :type "PrimitiveComponent Object Reference") (OtherActor :type "Actor Object Reference") (OtherComp :type "PrimitiveComponent Object Reference") (NormalImpulse :type "Vector Structure") (Hit :type "HitResult Structure (by ref)"))
  (if (and (`self.Overloaaded`) (`/Game/Blueprints/AC_Rotator.Moving` (`self.AC_Rotator`)) (== (`GameplayStatics.GetObjectClass` OtherActor) "/Game/Blueprints/Characters/BP_ThirdPersonCharacter.BP_ThirdPersonCharacter_C"))
    (message `/Game/Blueprints/BI_Ragdoll.EnableRagdoll` OtherActor (* (`SceneComponent.GetForwardVector` (`self.SM_Bld_Door_01`)) -1.0))))

(event `/Game/Blueprints/BI_Interactable.InteractStart`
  (params (TriggeringActor :type "Actor Object Reference") (TypeOfInteraction :type "/Game/Blueprints/Enum_InteractionType Enum" :default "NewEnumerator0"))
  (if (`/Game/Blueprints/AC_Rotator.Moving` (`self.AC_Rotator`))
    _
    (elif (== (`GameplayStatics.GetObjectClass` TriggeringActor) "/Game/Blueprints/Player/BP_Camera.BP_Camera_C")
      ;[1 1 1] Disable character interaction to prevent them from triggering the door right after the player has done so
      (`KismetSystemLibrary.K2_SetTimerDelegate` (delegate `EnableCharInteraction`) 1.0)
      (set `self.AllowCharacterInteraction` false)
      (set `self.TriggeringActor` TriggeringActor :!label _label)
      (switch `/Game/Blueprints/Enum_InteractionType` TypeOfInteraction
        (:`NewEnumerator0`
          (set `self.Overloaaded` false)
          (set `self.LerpSpeed` (`self.DefaultLerpSpeed`))
          (`self.TriggerOpen` :!label _label_2))
        (:`NewEnumerator1`
          (set `self.Overloaaded` true)
          (bind _success (`/Game/ThirdPerson/Blueprints/BP_ThirdPersonGameMode.TryUseEnergy` (`self.GameMode`) 30.0))
          (if _success
            (set `self.LerpSpeed` (* (`self.DefaultLerpSpeed`) (`self.OverloadFactor`)))
            (goto _label_2))))
      (elif (and (`self.AllowCharacterInteraction`) (not (`self.DoorOpen`)))
        (goto _label)))))

(event `EnableCharInteraction`
  ;[1 1 1] Disable character interaction to prevent them from triggering the door right after the player has done so
  (set `self.AllowCharacterInteraction` true))

(fn `GetHoverText`
  (returns (InteractText :type String) (OverloadText :type String) (BoobytrapText :type String))
  (if (`self.DoorOpen`)
    (return (`self.HoverTextClosed`) (`self.OverloadClosed`) "Press [Q] to boobytrap")
    (else
      (return (`self.HoverTextOpen`) (`self.OverloadOpen`) "Press [Q] to boobytrap"))))

(fn `IsInteractableThroughWalls`
  (returns (InteractableThroughWalls :type Boolean))
  (return false))

(fn `TriggerOpen`
  (if (not (`/Game/Blueprints/AC_Rotator.Moving` (`self.AC_Rotator`)))
    (if (`self.DoorOpen`)
      ;[1 1 1] Close door
      (set `self.TargetRotation` 0.0)
      (set `self.StartingRotation` (.yaw (.rotation (`SceneComponent.GetRelativeTransform` (`self.SM_Bld_Door_01`)))))
      (else
        ;[1 1 1] Open door away from triggering actor
        (`self.CheckClosestSide`
          (:`Left`
            (set `self.TargetRotation` (* (`self.MaxRotation`) -1.0)))
          (:`Right`
            (set `self.TargetRotation` (`self.MaxRotation`))))
        (set `self.StartingRotation` 0.0)))
    (set `self.DoorStatusUpdated` false)
    (`/Game/Blueprints/AC_Rotator.StartRotating` (`self.AC_Rotator`) (`self.LerpSpeed`) (`KismetMathLibrary.MakeRotator` 0.0 0.0 (`self.StartingRotation`)) (`KismetMathLibrary.MakeRotator` 0.0 0.0 (`self.TargetRotation`)))))

(fn `UserConstructionScript`)