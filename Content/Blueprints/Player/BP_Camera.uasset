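; BP_Camera is a possessable camera pawn that the player switches to by interacting with it, even through walls.
; InteractStart has the cached BP_Controller possess it, and its hover text shows the switch prompt.
; While possessed, it hides its cube body to clear the view and enables ticking on ACInteract, which is initialized with its Camera.
; Interact presses are forwarded to that component's current target, so the camera can trigger whatever it aims at.
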(event `self.ReceiveBeginPlay`
  (`/Game/Blueprints/Player/AC_Interact.Initialize` (`self.AC_Interact`) (`self.Camera`))
  (bind _asbp_controller (cast `/Game/Blueprints/Player/BP_Controller` (`GameplayStatics.GetPlayerController` 0)))
  (set `self.BP_Controller` _asbp_controller))

(event `self.ReceivePossessed`
  (params (NewController :type "Controller Object Reference"))
  ;[1 1 1] Enable/disable camera body to prevent it from blocking the view
  (`ActorComponent.SetComponentTickEnabled` (`self.AC_Interact`) true)
  (`SceneComponent.SetVisibility` (`self.Cube`) false true))

(event `self.ReceiveUnpossessed`
  (params (OldController :type "Controller Object Reference"))
  ;[1 1 1] Enable/disable camera body to prevent it from blocking the view
  (`ActorComponent.SetComponentTickEnabled` (`self.AC_Interact`) false)
  (`SceneComponent.SetVisibility` (`self.Cube`) true true))

(event `/Game/Blueprints/BI_Controllable.InteractPressed`
  (params (TypeOfInteraction :type "/Game/Blueprints/Enum_InteractionType Enum" :default "NewEnumerator0"))
  ;[1 1 1] Triggers interact on whatever this camera is aiming at
  (message `/Game/Blueprints/BI_Interactable.InteractStart` (`/Game/Blueprints/Player/AC_Interact.CurrentTarget` (`self.AC_Interact`)) self TypeOfInteraction))

(event `/Game/Blueprints/BI_Interactable.InteractStart`
  (params (TriggeringActor :type "Actor Object Reference") (TypeOfInteraction :type "/Game/Blueprints/Enum_InteractionType Enum" :default "NewEnumerator0"))
  ;[1 1 1] Switches view to this camera
  (`/Game/Blueprints/Player/BP_Controller.PossessNextPawn` (`self.BP_Controller`) self))

(fn `GetHoverText`
  (returns (InteractText :type String) (OverloadText :type String) (BoobytrapText :type String))
  (return "Press [E] to switch" "" ""))

(fn `IsInteractableThroughWalls`
  (returns (InteractableThroughWalls :type Boolean))
  (return true))

(fn `UserConstructionScript`)